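; BP_Grid is a grid actor that builds a tile field around its location from the configured shape, tile size and tile count.
; The construction script calls SpawnGrid, which clears and refills one InstancedStaticMesh, taking mesh, material and mesh size from DT_GridShapeData by shape name.
; It derives a snapped center and a bottom-left origin, then places scaled instances row by column.
; One shape flips tile yaw 180 degrees by index parity.
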(event EventBeginPlay)

(event Collision|EventActorBeginOverlap
  (params (OtherActor :type Actor%20Object%20Reference)))

(event EventTick
  (params (DeltaSeconds :type Float%20%28single-precision%29)))

(fn ConstructionScript
  (CallFunction|SpawnGrid (Transformation|GetActorLocation) (Variables|Default|GetGrid%20Tile%20Size) (Variables|Default|GetGrid%20Tile%20Count) (Variables|Default|GetGrid%20Shape)))

(fn SpawnGrid
  (params (CentralLocation :type Vector) (TileSize :type Vector) (TileCount :type Vector%202D%20Structure) (Shape :type E_GridShape%20Enum :default "NewEnumerator0"))
  (bind _returnvalue (CallFunction|GetCorectShapeData))
  (bind _instancedstaticmesh (Variables|Default|GetInstancedStaticMesh))
  (bind (_meshsize _mesh _meshmaterial _flatmesh _flatbordermaterial) (Utilities|Struct|BreakS_GridShapeData _returnvalue))
  (Variables|Default|SetGrid%20Central%20Location CentralLocation)
  (Variables|Default|SetGrid%20Tile%20Size TileSize)
  (Variables|Default|SetGrid%20Shape Shape)
  (Variables|Default|SetGrid%20Tile%20Count (Math|Vector2D|MakeVector2D (Math|Conversions|ToFloat(Integer) (Math|Float|Round (.x TileCount))) (Math|Conversions|ToFloat(Integer) (Math|Float|Round (.y TileCount)))))
  (CallFunction|DestroyGrid)
  (Components|StaticMesh|SetStaticMesh _instancedstaticmesh _flatmesh)
  (Rendering|Material|SetMaterial _instancedstaticmesh 0 _flatbordermaterial)
  (bind (_center _bottomleft) (CallFunction|CalculateCenterandBottomLeft))
  (Variables|Default|SetGrid%20Central%20Location _center)
  (Variables|Default|SetGridBottomLeftVorrectLocation _bottomleft)
  (for _index (range 0 (- (Math|Float|Round (.x (Variables|Default|GetGrid%20Tile%20Count))) 1))
    (LocalVariables|Setx _index)
    (for _index_2 (range 0 (- (Math|Float|Round (.y (Variables|Default|GetGrid%20Tile%20Count))) 1))
      (LocalVariables|Sety _index_2)
      (LocalVariables|SetIndex (Math|Vector2D|MakeVector2D (Math|Conversions|ToFloat(Integer) (LocalVariables|Getx)) (Math|Conversions|ToFloat(Integer) (LocalVariables|Gety))))
      (LocalVariables|SetTileTransform (Math|Transform|MakeTransform (CallFunction|GetTileLocationfromGridIndex (LocalVariables|GetIndex)) (CallFunction|GetTileRotationfromGridIndex (LocalVariables|GetIndex)) (/ (Variables|Default|GetGrid%20Tile%20Size) (.MeshSize (Utilities|Struct|BreakS_GridShapeData (CallFunction|GetCorectShapeData))))))
      (Components|InstancedStaticMesh|AddInstance (Variables|Default|GetInstancedStaticMesh) (LocalVariables|GetTileTransform) true))))

(fn GetCorectShapeData
  (bind _grid_shape (Variables|Default|GetGrid%20Shape))
  (bind _returnvalue (Utilities|String|EnumtoString _grid_shape))
  (bind _returnvalue_2 (Utilities|GetDataTableRow "/Game/Blueprint/Core/Grid/GridShapes/DT_GridShapeData.DT_GridShapeData" (Utilities|String|StringToName _returnvalue))
    (:then
      _)
    (:RowNotFound
      (Development|PrintString (Utilities|String|Append "Error - row not found -" _returnvalue) true true "(R=0.464000,G=0.000000,B=0.000000,A=1.000000)" 5.0)))
  (return _returnvalue_2))

(fn DestroyGrid
  (Components|InstancedStaticMesh|ClearInstances (Variables|Default|GetInstancedStaticMesh)))

(fn CalculateCenterandBottomLeft
  (bind _grid_tile_count (Variables|Default|GetGrid%20Tile%20Count))
  (LocalVariables|SetC (CallFunction|SnapVectortoVector (Variables|Default|GetGrid%20Central%20Location) (Variables|Default|GetGrid%20Tile%20Size)))
  (return (LocalVariables|GetC) (- (Variables|Default|GetGrid%20Central%20Location) (* (/ (- (Variables|Default|GetGrid%20Tile%20Count) (Math|Vector2D|MakeVector2D (Math|Float|SelectFloat 0.0 1.0 (CallFunction|IsFloatEvent (.x _grid_tile_count))) (Math|Float|SelectFloat 0.0 1.0 (CallFunction|IsFloatEvent (.y _grid_tile_count))))) "(X=2.000000,Y=0.000000)") (Variables|Default|GetGrid%20Tile%20Size)))))

(fn GetTileRotationfromGridIndex
  (params (GridIndex :type Vector%202D%20Structure))
  (if (Utilities|Enum|Equal(Enum) (Variables|Default|GetGrid%20Shape) "NewEnumerator0")
    (return (Math|Rotator|MakeRotator 0.0 0.0 (+ (Math|Float|SelectFloat 1.8e+02 0.0 (CallFunction|IsFloatEvent (.x GridIndex))) (Math|Float|SelectFloat 1.8e+02 0.0 (CallFunction|IsFloatEvent (.y GridIndex))))))
    (else
      (return ""))))

(fn GetTileLocationfromGridIndex
  (params (GridIndex :type Vector%202D%20Structure))
  (return (+ (Variables|Default|GetGridBottomLeftVorrectLocation) (* (Variables|Default|GetGrid%20Tile%20Size) (Math|Vector|MakeVector (Math|Conversions|ToFloat(Integer) (LocalVariables|Getx)) (Math|Conversions|ToFloat(Integer) (LocalVariables|Gety)) 0.0)))))