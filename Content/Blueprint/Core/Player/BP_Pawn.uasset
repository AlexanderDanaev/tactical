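; BP_Pawn is a player camera pawn with panning, spring-arm zoom and stepped rotation.
; Movement axes shift a target location along the pawn's forward and right vectors, the mouse wheel sets a clamped arm length, and rotation actions add 45-degree steps on release.
; Tick drives the pawn toward these targets with interp nodes, easing location and zoom without sweep collision; RInterpTo has no speed specified.
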(event EventTick
  (params (DeltaSeconds :type Float%20%28single-precision%29))
  (bind _springarm (Variables|Default|GetSpringArm))
  (Variables|/Script/Engine.SpringArmComponent|SetTargetArmLength _springarm (Math|Interpolation|FInterpTo (Variables|/Script/Engine.SpringArmComponent|GetTargetArmLength _springarm) (Variables|Default|GetZoomDessired) DeltaSeconds 2.0))
  (Transformation|SetActorLocation (Math|Interpolation|VInterpTo (Transformation|GetActorLocation) (Variables|Default|GetLocationDissared) DeltaSeconds 5.0) false false)
  (Transformation|SetActorRotation (Math|Interpolation|RInterpTo (Transformation|GetActorRotation) (Variables|Default|GetRotation_Dessired) DeltaSeconds 0.0)))

(event EventBeginPlay
  (Variables|Default|SetLocationDissared (Transformation|GetActorLocation))
  (Variables|Default|SetZoomDessired (Variables|/Script/Engine.SpringArmComponent|GetTargetArmLength (Variables|Default|GetSpringArm)))
  (Variables|Default|SetRotation_Dessired (Transformation|GetActorRotation)))

(event Input|ActionEvents|InputActionInputAction_RotationRight
  (params (Key :type Key%20Structure :default "None"))
  (:Released
    (Variables|Default|SetRotation_Dessired (Math|Rotator|CombineRotators (Variables|Default|GetRotation_Dessired) "0,-45.000000, 0"))))

(event Input|ActionEvents|InputActionInputAction_RotationLeft
  (params (Key :type Key%20Structure :default "None"))
  (:Released
    (Variables|Default|SetRotation_Dessired (Math|Rotator|CombineRotators (Variables|Default|GetRotation_Dessired) "0,45.000000, 0"))))

(event Input|AxisEvents|InputAxisInputAxisForward
  (params (AxisValue :type Float%20%28single-precision%29))
  (Variables|Default|SetLocationDissared (+ (Variables|Default|GetLocationDissared) (* (Transformation|GetActorForwardVector) (* AxisValue 2e+01)))))

(event Input|AxisEvents|InputAxisInputAxisRight
  (params (AxisValue :type Float%20%28single-precision%29))
  (Variables|Default|SetLocationDissared (+ (Variables|Default|GetLocationDissared) (* (Transformation|GetActorRightVector) (* AxisValue 2e+01)))))

(event Input|MouseEvents|MouseWheelAxis
  (params (AxisValue :type Float%20%28single-precision%29))
  (Variables|Default|SetZoomDessired (Math|Float|Clamp(Float) (+ (Variables|Default|GetZoomDessired) (* AxisValue 4e+01)) 1e+02 5e+03)))

(fn ConstructionScript)